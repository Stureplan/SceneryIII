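; BP_Consecration builds a ring of static meshes with matching Niagara effects, with no active gameplay logic.
; The construction script uses sine and cosine to space MeshNumber-driven components at Distance from the root, lowered vertically and rotated toward the center.
; Each Niagara component receives its paired mesh through the MeshShoulders variable.
; The root's world location is written to MPC_Wind as CenterPosition, exposing the ring's center to materials.
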(event EventBeginPlay)

(event Collision|EventActorBeginOverlap
  (params (OtherActor :type Actor%20Object%20Reference)))

(event EventTick
  (params (DeltaSeconds :type Float%20%28single-precision%29)))

(fn ConstructionScript
  (bind _defaultsceneroot (Variables|Default|GetDefaultSceneRoot))
  (bind _returnvalue (Transformation|GetWorldLocation _defaultsceneroot))
  (for _index (range 0 (Variables|Default|GetMeshNumber))
    (bind _returnvalue_2 (AddComponent|AddStaticMeshComponent false (Math|Transform|MakeTransform (+ (* (Math|Vector|MakeVector (Math|Trig|Cos(Radians) (* _index (* (Math|Float|MakeLiteralFloat 2.0) (/ (Math|Float|MakeLiteralFloat 3.14) (Variables|Default|GetMeshNumber))))) (Math|Trig|Sin(Radians) (* _index (* (Math|Float|MakeLiteralFloat 2.0) (/ (Math|Float|MakeLiteralFloat 3.14) (Variables|Default|GetMeshNumber))))) 0.0) (Variables|Default|GetDistance)) "0.000000,0.000000,-250.000000") (Math|Rotator|FindLookatRotation (+ (* (Math|Vector|MakeVector (Math|Trig|Cos(Radians) (* _index (* (Math|Float|MakeLiteralFloat 2.0) (/ (Math|Float|MakeLiteralFloat 3.14) (Variables|Default|GetMeshNumber))))) (Math|Trig|Sin(Radians) (* _index (* (Math|Float|MakeLiteralFloat 2.0) (/ (Math|Float|MakeLiteralFloat 3.14) (Variables|Default|GetMeshNumber))))) 0.0) (Variables|Default|GetDistance)) _returnvalue) _returnvalue))))
    (bind _returnvalue_3 (AddComponent|AddNiagaraComponent false (Math|Transform|MakeTransform (+ (* (Math|Vector|MakeVector (Math|Trig|Cos(Radians) (* _index (* (Math|Float|MakeLiteralFloat 2.0) (/ (Math|Float|MakeLiteralFloat 3.14) (Variables|Default|GetMeshNumber))))) (Math|Trig|Sin(Radians) (* _index (* (Math|Float|MakeLiteralFloat 2.0) (/ (Math|Float|MakeLiteralFloat 3.14) (Variables|Default|GetMeshNumber))))) 0.0) (Variables|Default|GetDistance)) "0.000000,0.000000,-250.000000") (Math|Rotator|FindLookatRotation (+ (* (Math|Vector|MakeVector (Math|Trig|Cos(Radians) (* _index (* (Math|Float|MakeLiteralFloat 2.0) (/ (Math|Float|MakeLiteralFloat 3.14) (Variables|Default|GetMeshNumber))))) (Math|Trig|Sin(Radians) (* _index (* (Math|Float|MakeLiteralFloat 2.0) (/ (Math|Float|MakeLiteralFloat 3.14) (Variables|Default|GetMeshNumber))))) 0.0) (Variables|Default|GetDistance)) _returnvalue) _returnvalue))))
    (Class|NiagaraComponent|SetVariableStaticMesh _returnvalue_3 "MeshShoulders" (Variables|/Script/Engine.StaticMeshComponent|GetStaticMesh _returnvalue_2))
    (Rendering|Material|SetVectorParameterValue "/Game/Materials/MPC_Wind.MPC_Wind" "CenterPosition" (Math|Conversions|ToLinearColor(Vector) (Transformation|GetWorldLocation (Variables|Default|GetDefaultSceneRoot))) :!class /Script/Engine.KismetMaterialLibrary)))