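; BP_Blood is a looping blood effect that drives a Niagara system along two splines.
; After a startup delay, a timeline samples both splines and feeds local positions, rotations as quaternions and a progress value into Niagara each update.
; It also writes Spline01's world height to the MPC_Blood_Demon material parameter collection.
; When the timeline finishes, Niagara deactivates and the cycle restarts after a short pause.
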(event Custom|Start
  (Utilities|FlowControl|Sequence
    (:then_0
      (Components|Activation|Activate (Variables|Default|GetNiagara) true))
    (:then_1
      (bind (_direction _time _progress) (Timeline|Timeline Stop)
        (:Update
          (Niagara|SetNiagaraVariable(Vector3) (Variables|Default|GetNiagara) "TargetVector_01" (+ (Spline|GetLocationatTime (Variables|Default|GetSpline_01) (* _time (Variables|/Script/Engine.SplineComponent|GetDuration (Variables|Default|GetSpline_01))) "Local" true) (Variables|/Script/Engine.SceneComponent|GetRelativeLocation (Variables|Default|GetSpline_01))))
          (Niagara|SetNiagaraVariable(Vector3) (Variables|Default|GetNiagara) "TargetVector_02" (+ (Spline|GetLocationatTime (Variables|Default|GetSpline_02) (* _time (Variables|/Script/Engine.SplineComponent|GetDuration (Variables|Default|GetSpline_01))) "Local" true) (Variables|/Script/Engine.SceneComponent|GetRelativeLocation (Variables|Default|GetSpline_02))))
          (Niagara|SetNiagaraVariable(Float) (Variables|Default|GetNiagara) "SplineProgress" _progress)
          (Rendering|Material|SetScalarParameterValue "/Game/Materials/MPC_Blood_Demon.MPC_Blood_Demon" "TargetHeight" (.Z (Class|KismetMathLibrary|BreakVector3f (Spline|GetLocationatTime (Variables|Default|GetSpline_01) (* _time (Variables|/Script/Engine.SplineComponent|GetDuration (Variables|Default|GetSpline_01))) "World" true))) :!class /Script/Engine.KismetMaterialLibrary)
          (Class|NiagaraComponent|SetVariableQuat (Variables|Default|GetNiagara) "TargetQuat_01" (Math|Conversions|ToQuaternion(Rotator) (Class|SplineComponent|GetRotationatTime (Variables|Default|GetSpline_01) (* _time (Variables|/Script/Engine.SplineComponent|GetDuration (Variables|Default|GetSpline_01))) "Local" false)))
          (Class|NiagaraComponent|SetVariableQuat (Variables|Default|GetNiagara) "TargetQuat_02" (Math|Conversions|ToQuaternion(Rotator) (Class|SplineComponent|GetRotationatTime (Variables|Default|GetSpline_02) (* _time (Variables|/Script/Engine.SplineComponent|GetDuration (Variables|Default|GetSpline_01))) "Local" false))))
        (:Finished
          (Components|Activation|Deactivate (Variables|Default|GetNiagara))
          (Utilities|FlowControl|Delay 2.0)
          (CallFunction|Start))))
    (:then_2
      (Timeline|Timeline PlayFromStart))))

(event EventBeginPlay
  (Utilities|FlowControl|Delay 2.0)
  (Variables|/Script/Engine.SplineComponent|SetDuration (Variables|Default|GetSpline_01) (Components|Timeline|GetTimelineLength (Variables|Default|GetTimeline)))
  (Variables|/Script/Engine.SplineComponent|SetDuration (Variables|Default|GetSpline_02) (Components|Timeline|GetTimelineLength (Variables|Default|GetTimeline)))
  (CallFunction|Start))

(fn ConstructionScript)